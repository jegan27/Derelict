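; Ceiling lights Blueprint for a sci-fi environment, grouping two sets of emissive fixture meshes with spotlights and offering Flicker and GoEmergency events.
; The construction script creates dynamic material instances for both fixture sets so their glow can change at runtime.
; Flicker toggles glow and spotlights off and on using a delay and counter loop, ending lit.
; GoEmergency darkens the ceiling panels, turns the other fixtures red and dims the spotlights to red.
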(event Custom|Flicker
  (bind _flickerduration (Variables|Default|GetFlickerDuration))
  (Rendering|Material|SetScalarParameterValue (Variables|Default|GetLightDynMat01) "illuminationIntensity" 0.0 :!class /Script/Engine.MaterialInstanceDynamic :!label _label)
  (Rendering|Material|SetScalarParameterValue (Variables|Default|GetCeilDynMat01) "illuminationIntensity" 0.0 :!class /Script/Engine.MaterialInstanceDynamic)
  (Rendering|Components|Light|SetIntensity (Variables|Default|GetSpotLight9_0) 0.0)
  (Utilities|FlowControl|Delay _flickerduration)
  (Rendering|Material|SetScalarParameterValue (Variables|Default|GetLightDynMat01) "illuminationIntensity" 4.0 :!class /Script/Engine.MaterialInstanceDynamic)
  (Rendering|Material|SetScalarParameterValue (Variables|Default|GetCeilDynMat01) "illuminationIntensity" 4.0 :!class /Script/Engine.MaterialInstanceDynamic)
  (Rendering|Components|Light|SetIntensity (Variables|Default|GetSpotLight9_0) 3e+04)
  (Variables|Default|SetflickerCounter (+ (Variables|Default|GetflickerCounter) 1))
  (Math|Integer|CompareInt (Variables|Default|GetflickerCounter) 15
    (:>
      _)
    (:==
      _)
    (:<
      (Utilities|FlowControl|Delay _flickerduration)
      (goto _label)))
  (Rendering|Material|SetScalarParameterValue (Variables|Default|GetLightDynMat01) "illuminationIntensity" 4.0 :!class /Script/Engine.MaterialInstanceDynamic)
  (Rendering|Material|SetScalarParameterValue (Variables|Default|GetCeilDynMat01) "illuminationIntensity" 4.0 :!class /Script/Engine.MaterialInstanceDynamic)
  (Rendering|Components|Light|SetIntensity (Variables|Default|GetSpotLight9_0) 3e+04))

(event Custom|GoEmergency
  (Rendering|Material|SetScalarParameterValue (Variables|Default|GetLightDynMat01) "illuminationIntensity" 4.0 :!class /Script/Engine.MaterialInstanceDynamic)
  (Rendering|Material|SetVectorParameterValue (Variables|Default|GetLightDynMat01) "illuminationColor" "(R=1.000000,G=0.000000,B=0.000000,A=1.000000)" :!class /Script/Engine.MaterialInstanceDynamic)
  (Rendering|Material|SetScalarParameterValue (Variables|Default|GetCeilDynMat01) "illuminationIntensity" 0.0 :!class /Script/Engine.MaterialInstanceDynamic)
  (Rendering|Components|Light|SetIntensity (Variables|Default|GetSpotLight9_0) 6.5e+03)
  (Rendering|Components|Light|SetLightColor (Variables|Default|GetSpotLight9_0) "(R=0.520000,G=0.000000,B=0.064012,A=1.000000)" true))

(event EventBeginPlay)

(fn ConstructionScript
  (bind _returnvalue (Rendering|Material|CreateDynamicMaterialInstance (Variables|Default|GetDH_LVL_CeilingLight_SM10_0) 0 "/Game/SciFiEnvironmentSet/Materials/DH_CeilingLight_Mat2.DH_CeilingLight_Mat2" :!class /Script/Engine.PrimitiveComponent))
  (Variables|Default|SetCeilDynMat01 _returnvalue)
  (bind _returnvalue_2 (Rendering|Material|CreateDynamicMaterialInstance (Variables|Default|GetDH_LVL_CeilingLight_SM16_0) 0 "/Game/SciFiEnvironmentSet/Materials/DH_CeilingLight_Mat2.DH_CeilingLight_Mat2" :!class /Script/Engine.PrimitiveComponent))
  (Variables|Default|SetCeilDynMat02 _returnvalue_2)
  (bind _returnvalue_3 (Rendering|Material|CreateDynamicMaterialInstance (Variables|Default|GetDH_LVL_CeilingLight_SM15_0) 0 "/Game/SciFiEnvironmentSet/Materials/DH_CeilingLight_Mat2.DH_CeilingLight_Mat2" :!class /Script/Engine.PrimitiveComponent))
  (Variables|Default|SetCeilDynMat03 _returnvalue_3)
  (bind _returnvalue_4 (Rendering|Material|CreateDynamicMaterialInstance (Variables|Default|GetDH_LVL_CeilingLight_SM14_0) 0 "/Game/SciFiEnvironmentSet/Materials/DH_CeilingLight_Mat2.DH_CeilingLight_Mat2" :!class /Script/Engine.PrimitiveComponent))
  (Variables|Default|SetCeilDynMat04 _returnvalue_4)
  (bind _returnvalue_5 (Rendering|Material|CreateDynamicMaterialInstance (Variables|Default|GetDH_LVL_CeilingLight_SM13_0) 0 "/Game/SciFiEnvironmentSet/Materials/DH_CeilingLight_Mat2.DH_CeilingLight_Mat2" :!class /Script/Engine.PrimitiveComponent))
  (Variables|Default|SetCeilDynMat05 _returnvalue_5)
  (bind _returnvalue_6 (Rendering|Material|CreateDynamicMaterialInstance (Variables|Default|GetDH_LVL_CeilingLight_SM12_0) 0 "/Game/SciFiEnvironmentSet/Materials/DH_CeilingLight_Mat2.DH_CeilingLight_Mat2" :!class /Script/Engine.PrimitiveComponent))
  (Variables|Default|SetCeilDynMat06 _returnvalue_6)
  (bind _returnvalue_7 (Rendering|Material|CreateDynamicMaterialInstance (Variables|Default|GetDH_LVL_CeilingLight_SM9_0) 0 "/Game/SciFiEnvironmentSet/Materials/DH_CeilingLight_Mat2.DH_CeilingLight_Mat2" :!class /Script/Engine.PrimitiveComponent))
  (Variables|Default|SetCeilDynMat07 _returnvalue_7)
  (bind _returnvalue_8 (Rendering|Material|CreateDynamicMaterialInstance (Variables|Default|GetDH_E2_Lights04_SM7_0) 0 "/Game/SciFiEnvironmentSet/Materials/DH_Lights02_Mat.DH_Lights02_Mat" :!class /Script/Engine.PrimitiveComponent))
  (Variables|Default|SetLightDynMat01 _returnvalue_8)
  (bind _returnvalue_9 (Rendering|Material|CreateDynamicMaterialInstance (Variables|Default|GetDH_E2_Lights04_SM6_0) 0 "/Game/SciFiEnvironmentSet/Materials/DH_Lights02_Mat.DH_Lights02_Mat" :!class /Script/Engine.PrimitiveComponent))
  (Variables|Default|SetLightDynMat02 _returnvalue_9)
  (bind _returnvalue_10 (Rendering|Material|CreateDynamicMaterialInstance (Variables|Default|GetDH_E2_Lights04_SM5_0) 0 "/Game/SciFiEnvironmentSet/Materials/DH_Lights02_Mat.DH_Lights02_Mat" :!class /Script/Engine.PrimitiveComponent))
  (Variables|Default|SetLightDynMat03 _returnvalue_10)
  (bind _returnvalue_11 (Rendering|Material|CreateDynamicMaterialInstance (Variables|Default|GetDH_E2_Lights04_SM4_0) 0 "/Game/SciFiEnvironmentSet/Materials/DH_Lights02_Mat.DH_Lights02_Mat" :!class /Script/Engine.PrimitiveComponent))
  (Variables|Default|SetLightDynMat04 _returnvalue_11)
  (bind _returnvalue_12 (Rendering|Material|CreateDynamicMaterialInstance (Variables|Default|GetDH_E2_Lights04_SM3_0) 0 "/Game/SciFiEnvironmentSet/Materials/DH_Lights02_Mat.DH_Lights02_Mat" :!class /Script/Engine.PrimitiveComponent))
  (Variables|Default|SetLightDynMat05 _returnvalue_12)
  (bind _returnvalue_13 (Rendering|Material|CreateDynamicMaterialInstance (Variables|Default|GetDH_E2_Lights04_SM2_0) 0 "/Game/SciFiEnvironmentSet/Materials/DH_Lights02_Mat.DH_Lights02_Mat" :!class /Script/Engine.PrimitiveComponent))
  (Variables|Default|SetLightDynMat06 _returnvalue_13))
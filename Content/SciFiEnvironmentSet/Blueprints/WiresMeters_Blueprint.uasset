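; Sci-fi environment prop Blueprint that groups living room wire meshes with spot lights.
; The construction script creates a dynamic instance of LivingRoomWire_Mat for each of six wire meshes and stores them as variables.
; An unconnected Event Graph chain would zero the materials' illuminationIntensity and the intensity of six spot lights.
; BeginPlay is empty, so nothing changes the glow or lights at runtime.
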(event EventBeginPlay)

(fn ConstructionScript
  (bind _returnvalue (Rendering|Material|CreateDynamicMaterialInstance (Variables|Default|GetDH_E1C7_livingroom_Wires_SM_6_0) 0 "/Game/Developers/SHASHANK/SciFi/Materials/LivingRoomWire_Mat.LivingRoomWire_Mat" :!class /Script/Engine.PrimitiveComponent))
  (Variables|Default|SetDynMat01 _returnvalue)
  (bind _returnvalue_2 (Rendering|Material|CreateDynamicMaterialInstance (Variables|Default|GetDH_E1C7_livingroom_Wires_SM_9_0) 0 "/Game/Developers/SHASHANK/SciFi/Materials/LivingRoomWire_Mat.LivingRoomWire_Mat" :!class /Script/Engine.PrimitiveComponent))
  (Variables|Default|SetDynMat02 _returnvalue_2)
  (bind _returnvalue_3 (Rendering|Material|CreateDynamicMaterialInstance (Variables|Default|GetDH_E1C7_livingroom_Wires_SM_10_0) 0 "/Game/Developers/SHASHANK/SciFi/Materials/LivingRoomWire_Mat.LivingRoomWire_Mat" :!class /Script/Engine.PrimitiveComponent))
  (Variables|Default|SetDynMat03 _returnvalue_3)
  (bind _returnvalue_4 (Rendering|Material|CreateDynamicMaterialInstance (Variables|Default|GetDH_E1C7_livingroom_Wires_SM_5_0) 0 "/Game/Developers/SHASHANK/SciFi/Materials/LivingRoomWire_Mat.LivingRoomWire_Mat" :!class /Script/Engine.PrimitiveComponent))
  (Variables|Default|SetDynMat04 _returnvalue_4)
  (bind _returnvalue_5 (Rendering|Material|CreateDynamicMaterialInstance (Variables|Default|GetDH_E1C7_livingroom_Wires_SM_7_0) 0 "/Game/Developers/SHASHANK/SciFi/Materials/LivingRoomWire_Mat.LivingRoomWire_Mat" :!class /Script/Engine.PrimitiveComponent))
  (Variables|Default|SetDynMat05 _returnvalue_5)
  (bind _returnvalue_6 (Rendering|Material|CreateDynamicMaterialInstance (Variables|Default|GetDH_E1C7_livingroom_Wires_SM_8_0) 0 "/Game/Developers/SHASHANK/SciFi/Materials/LivingRoomWire_Mat.LivingRoomWire_Mat" :!class /Script/Engine.PrimitiveComponent))
  (Variables|Default|SetDynMat06 _returnvalue_6))
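; AutoDoors01 is an automatic sliding double door that opens on trigger overlap and shuts when the overlap ends.
; One timeline alpha lerps both panels from their relative origin to separate left and right open offsets, reversing to close.
; Opening also activates a component, which shutting deactivates.
; OpenDoor and ShutDoor events share the same logic as the trigger.
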(event OnComponentBeginOverlap(Trigger)
  (params (OtherActor :type Actor%20Object%20Reference) (OtherComp :type Primitive%20Component%20Object%20Reference) (OtherBodyIndex :type Integer) (bFromSweep :type Boolean) (SweepResult :type Hit%20Result%20Structure%20%28by%20ref%29))
  (Components|Activation|Activate false)
  (bind _doorseqleft (Timeline|Timeline_LeftDoor Play)
    (:Update
      (Transformation|SetRelativeLocation (Math|Vector|Lerp(Vector) "0, 0, 0" (Variables|Default|GetDoorOpen_Left) _doorseqleft) false false)
      (Transformation|SetRelativeLocation (Math|Vector|Lerp(Vector) "0, 0, 0" (Variables|Default|GetDoorOpen_Right) _doorseqleft) false false))))

(event OnComponentEndOverlap(Trigger)
  (params (OtherActor :type Actor%20Object%20Reference) (OtherComp :type Primitive%20Component%20Object%20Reference) (OtherBodyIndex :type Integer))
  (Components|Activation|Deactivate)
  (bind _doorseqleft (Timeline|Timeline_LeftDoor Reverse)
    (:Update
      (Transformation|SetRelativeLocation (Math|Vector|Lerp(Vector) "0, 0, 0" (Variables|Default|GetDoorOpen_Left) _doorseqleft) false false)
      (Transformation|SetRelativeLocation (Math|Vector|Lerp(Vector) "0, 0, 0" (Variables|Default|GetDoorOpen_Right) _doorseqleft) false false))))

(event Custom|OpenDoor
  (Components|Activation|Activate false)
  (bind _doorseqleft (Timeline|Timeline_LeftDoor Play)
    (:Update
      (Transformation|SetRelativeLocation (Math|Vector|Lerp(Vector) "0, 0, 0" (Variables|Default|GetDoorOpen_Left) _doorseqleft) false false)
      (Transformation|SetRelativeLocation (Math|Vector|Lerp(Vector) "0, 0, 0" (Variables|Default|GetDoorOpen_Right) _doorseqleft) false false))))

(event Custom|ShutDoor
  (Components|Activation|Deactivate)
  (bind _doorseqleft (Timeline|Timeline_LeftDoor Reverse)
    (:Update
      (Transformation|SetRelativeLocation (Math|Vector|Lerp(Vector) "0, 0, 0" (Variables|Default|GetDoorOpen_Left) _doorseqleft) false false)
      (Transformation|SetRelativeLocation (Math|Vector|Lerp(Vector) "0, 0, 0" (Variables|Default|GetDoorOpen_Right) _doorseqleft) false false))))

(fn ConstructionScript)
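; Generator Blueprint for a sci-fi environment prop that animates its spotlights and emissive material through different power states.
; BeginPlay runs a timeline that shifts four main spotlights between high and low intensity, and StopCycle halts it.
; Reaction blends those lights and a halogen group toward reaction intensities, while GoDark fades all to zero.
; GoDark also zeroes illumination parameters on a dynamic material instance created in the construction script.
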(event Custom|StopCycle
  (bind _switch (Timeline|Timeline_0 Stop)
    (:Update
      (Rendering|Components|Light|SetIntensity (Variables|Default|GetSpotLight50_0) (Math|Interpolation|Ease "Linear" _switch (Variables|Default|GetLights_HighIntensity) (Variables|Default|GetLights_LowIntensity)))
      (Rendering|Components|Light|SetIntensity (Variables|Default|GetSpotLight51_0) (Math|Interpolation|Ease "Linear" _switch (Variables|Default|GetLights_HighIntensity) (Variables|Default|GetLights_LowIntensity)))
      (Rendering|Components|Light|SetIntensity (Variables|Default|GetSpotLight52_0) (Math|Interpolation|Ease "Linear" _switch (Variables|Default|GetLights_HighIntensity) (Variables|Default|GetLights_LowIntensity)))
      (Rendering|Components|Light|SetIntensity (Variables|Default|GetSpotLight53_0) (Math|Interpolation|Ease "Linear" _switch (Variables|Default|GetLights_HighIntensity) (Variables|Default|GetLights_LowIntensity))))))

(event Custom|GoDark
  (bind _gen_dynmat (Variables|Default|GetGen_DynMat))
  (bind _reactiontime (Timeline|Timeline_2 Play)
    (:Update
      (Rendering|Components|Light|SetIntensity (Variables|Default|GetSpotLight50_0) (Math|Float|Lerp (Variables|Default|GetLights_HighIntensity) 0.0 _reactiontime))
      (Rendering|Components|Light|SetIntensity (Variables|Default|GetSpotLight61_0) (Math|Float|Lerp (Variables|Default|GetHalogenLights_NormalIntensity) 0.0 _reactiontime))
      (Rendering|Material|SetScalarParameterValue _gen_dynmat "flashLights_IlluminationIntensity" 0.0 :!class /Script/Engine.MaterialInstanceDynamic)
      (Rendering|Material|SetScalarParameterValue _gen_dynmat "reactor_IlluminationIntensity" 0.0 :!class /Script/Engine.MaterialInstanceDynamic)
      (Rendering|Material|SetScalarParameterValue _gen_dynmat "screens_IlluminationIntensity" 0.0 :!class /Script/Engine.MaterialInstanceDynamic))))

(event Custom|Reaction
  (bind _reactiontime (Timeline|Timeline_1 PlayFromStart)
    (:Update
      (Rendering|Components|Light|SetIntensity (Variables|Default|GetSpotLight50_0) (Math|Float|Lerp (Variables|Default|GetLights_HighIntensity) (Variables|Default|GetLights_Reaction) _reactiontime))
      (Rendering|Components|Light|SetIntensity (Variables|Default|GetSpotLight61_0) (Math|Float|Lerp (Variables|Default|GetHalogenLights_NormalIntensity) (Variables|Default|GetHalogenLights_ReactionIntensity) _reactiontime)))))

(event EventBeginPlay
  (bind _switch (Timeline|Timeline_0 Play)
    (:Update
      (Rendering|Components|Light|SetIntensity (Variables|Default|GetSpotLight50_0) (Math|Interpolation|Ease "Linear" _switch (Variables|Default|GetLights_HighIntensity) (Variables|Default|GetLights_LowIntensity)))
      (Rendering|Components|Light|SetIntensity (Variables|Default|GetSpotLight51_0) (Math|Interpolation|Ease "Linear" _switch (Variables|Default|GetLights_HighIntensity) (Variables|Default|GetLights_LowIntensity)))
      (Rendering|Components|Light|SetIntensity (Variables|Default|GetSpotLight52_0) (Math|Interpolation|Ease "Linear" _switch (Variables|Default|GetLights_HighIntensity) (Variables|Default|GetLights_LowIntensity)))
      (Rendering|Components|Light|SetIntensity (Variables|Default|GetSpotLight53_0) (Math|Interpolation|Ease "Linear" _switch (Variables|Default|GetLights_HighIntensity) (Variables|Default|GetLights_LowIntensity))))))

(fn ConstructionScript
  (bind _returnvalue (Rendering|Material|CreateDynamicMaterialInstance (Variables|Default|GetGenerator_0) 0 "/Game/SciFiEnvironmentSet/Materials/Generator_Mat.Generator_Mat" :!class /Script/Engine.PrimitiveComponent))
  (Variables|Default|SetGen_DynMat _returnvalue))
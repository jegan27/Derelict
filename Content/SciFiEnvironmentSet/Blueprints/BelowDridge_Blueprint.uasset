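; Environment lighting Blueprint that controls eight light fixtures and their spotlights, with flicker and blackout effects.
; The construction script gives each fixture mesh a dynamic material instance, whose illumination parameter switches alongside spotlight intensity.
; Flicker and GoDark loop through delayed off/on pulses, ending lit and dark respectively, while GoDark02 cuts power instantly.
; Both loops share a FlickerCounter that is never reset here.
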(event Custom|GoDark02
  (Rendering|Material|SetScalarParameterValue (Variables|Default|GetDynMat01) "illuminationIntensity" 0.0 :!class /Script/Engine.MaterialInstanceDynamic)
  (Rendering|Components|Light|SetIntensity (Variables|Default|GetSpotLight36_0) 0.0))

(event Custom|GoDark
  (Rendering|Material|SetScalarParameterValue (Variables|Default|GetDynMat01) "illuminationIntensity" 0.0 :!class /Script/Engine.MaterialInstanceDynamic :!label _label)
  (Rendering|Components|Light|SetIntensity (Variables|Default|GetSpotLight36_0) 0.0)
  (Utilities|FlowControl|Delay (Variables|Default|GetFlickerDuration))
  (Rendering|Material|SetScalarParameterValue (Variables|Default|GetDynMat01) "illuminationIntensity" 6.0 :!class /Script/Engine.MaterialInstanceDynamic)
  (Rendering|Components|Light|SetIntensity (Variables|Default|GetSpotLight36_0) 1.1e+04)
  (Variables|Default|SetflickerCounter (+ (Variables|Default|GetflickerCounter) 1))
  (Math|Integer|CompareInt (Variables|Default|GetflickerCounter) 20
    (:>
      _)
    (:==
      _)
    (:<
      (Utilities|FlowControl|Delay 0.2)
      (goto _label)))
  (Rendering|Material|SetScalarParameterValue (Variables|Default|GetDynMat01) "illuminationIntensity" 0.0 :!class /Script/Engine.MaterialInstanceDynamic)
  (Rendering|Components|Light|SetIntensity (Variables|Default|GetSpotLight36_0) 0.0))

(event Custom|Flicker
  (Rendering|Material|SetScalarParameterValue (Variables|Default|GetDynMat01) "illuminationIntensity" 0.0 :!class /Script/Engine.MaterialInstanceDynamic :!label _label)
  (Rendering|Components|Light|SetIntensity (Variables|Default|GetSpotLight36_0) 0.0)
  (Utilities|FlowControl|Delay (Variables|Default|GetFlickerDuration))
  (Rendering|Material|SetScalarParameterValue (Variables|Default|GetDynMat01) "illuminationIntensity" 6.0 :!class /Script/Engine.MaterialInstanceDynamic)
  (Rendering|Components|Light|SetIntensity (Variables|Default|GetSpotLight36_0) 1.1e+04)
  (Variables|Default|SetflickerCounter (+ (Variables|Default|GetflickerCounter) 1))
  (Math|Integer|CompareInt (Variables|Default|GetflickerCounter) 20
    (:>
      _)
    (:==
      _)
    (:<
      (Utilities|FlowControl|Delay 0.2)
      (goto _label)))
  (Rendering|Material|SetScalarParameterValue (Variables|Default|GetDynMat01) "illuminationIntensity" 6.0 :!class /Script/Engine.MaterialInstanceDynamic)
  (Rendering|Components|Light|SetIntensity (Variables|Default|GetSpotLight36_0) 1.1e+04))

(event EventBeginPlay)

(fn ConstructionScript
  (bind _returnvalue (Rendering|Material|CreateDynamicMaterialInstance (Variables|Default|GetDH_LVL_Light01_SM_12_0) 0 "/Game/Developers/SHASHANK/SciFi/Materials/DH_Light01_Mat.DH_Light01_Mat" :!class /Script/Engine.PrimitiveComponent))
  (Variables|Default|SetDynMat01 _returnvalue)
  (bind _returnvalue_2 (Rendering|Material|CreateDynamicMaterialInstance (Variables|Default|GetDH_LVL_Light01_SM_11_0) 0 "/Game/Developers/SHASHANK/SciFi/Materials/DH_Light01_Mat.DH_Light01_Mat" :!class /Script/Engine.PrimitiveComponent))
  (Variables|Default|SetDynMat02 _returnvalue_2)
  (bind _returnvalue_3 (Rendering|Material|CreateDynamicMaterialInstance (Variables|Default|GetDH_LVL_Light01_SM_6_0) 0 "/Game/Developers/SHASHANK/SciFi/Materials/DH_Light01_Mat.DH_Light01_Mat" :!class /Script/Engine.PrimitiveComponent))
  (Variables|Default|SetDynMat03 _returnvalue_3)
  (bind _returnvalue_4 (Rendering|Material|CreateDynamicMaterialInstance (Variables|Default|GetDH_LVL_Light01_SM_10_0) 0 "/Game/Developers/SHASHANK/SciFi/Materials/DH_Light01_Mat.DH_Light01_Mat" :!class /Script/Engine.PrimitiveComponent))
  (Variables|Default|SetDynMat04 _returnvalue_4)
  (bind _returnvalue_5 (Rendering|Material|CreateDynamicMaterialInstance (Variables|Default|GetDH_LVL_Light01_SM_13_0) 0 "/Game/Developers/SHASHANK/SciFi/Materials/DH_Light01_Mat.DH_Light01_Mat" :!class /Script/Engine.PrimitiveComponent))
  (Variables|Default|SetDynMat05 _returnvalue_5)
  (bind _returnvalue_6 (Rendering|Material|CreateDynamicMaterialInstance (Variables|Default|GetDH_LVL_Light01_SM_14_0) 0 "/Game/Developers/SHASHANK/SciFi/Materials/DH_Light01_Mat.DH_Light01_Mat" :!class /Script/Engine.PrimitiveComponent))
  (Variables|Default|SetDynMat06 _returnvalue_6)
  (bind _returnvalue_7 (Rendering|Material|CreateDynamicMaterialInstance (Variables|Default|GetDH_LVL_Light01_SM_3_0) 0 "/Game/Developers/SHASHANK/SciFi/Materials/DH_Light01_Mat.DH_Light01_Mat" :!class /Script/Engine.PrimitiveComponent))
  (Variables|Default|SetDynMat07 _returnvalue_7)
  (bind _returnvalue_8 (Rendering|Material|CreateDynamicMaterialInstance (Variables|Default|GetDH_LVL_Light01_SM_4_0) 0 "/Game/Developers/SHASHANK/SciFi/Materials/DH_Light01_Mat.DH_Light01_Mat" :!class /Script/Engine.PrimitiveComponent))
  (Variables|Default|SetDynMat08 _returnvalue_8))
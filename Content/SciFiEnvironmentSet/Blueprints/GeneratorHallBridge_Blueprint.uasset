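; Generator hall bridge Blueprint that controls ten arch lights, with events to flicker them on, flicker them dark or cut them instantly.
; The construction script creates dynamic material instances so events drive emissive intensity alongside spotlight intensity.
; Flicker and GoDark loop via Delay until a shared, never-reset FlickerCounter reaches ten, then settle bright or dark respectively.
; GoDark02 switches everything off immediately; BeginPlay does nothing.
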(event Custom|GoDark02
  (Rendering|Material|SetScalarParameterValue (Variables|Default|GetDynMat) "illuminationIntensity" 0.0 :!class /Script/Engine.MaterialInstanceDynamic)
  (Rendering|Components|Light|SetIntensity (Variables|Default|GetSpotLight10_0) 0.0))

(event Custom|Flicker
  (bind _flickerduration (Variables|Default|GetflickerDuration))
  (Rendering|Material|SetScalarParameterValue (Variables|Default|GetDynMat) "illuminationIntensity" 0.0 :!class /Script/Engine.MaterialInstanceDynamic :!label _label)
  (Rendering|Components|Light|SetIntensity (Variables|Default|GetSpotLight10_0) 0.0)
  (Utilities|FlowControl|Delay _flickerduration)
  (Rendering|Material|SetScalarParameterValue (Variables|Default|GetDynMat) "illuminationIntensity" 4.0 :!class /Script/Engine.MaterialInstanceDynamic)
  (Rendering|Components|Light|SetIntensity (Variables|Default|GetSpotLight10_0) 2.5e+03)
  (Utilities|FlowControl|Delay _flickerduration)
  (Variables|Default|SetflickerCounter (+ (Variables|Default|GetflickerCounter) 1))
  (Math|Integer|CompareInt (Variables|Default|GetflickerCounter) 10
    (:>
      _)
    (:==
      _)
    (:<
      (goto _label)))
  (Rendering|Material|SetScalarParameterValue (Variables|Default|GetDynMat) "illuminationIntensity" 4.0 :!class /Script/Engine.MaterialInstanceDynamic)
  (Rendering|Components|Light|SetIntensity (Variables|Default|GetSpotLight10_0) 1e+04))

(event Custom|GoDark
  (bind _flickerduration (Variables|Default|GetflickerDuration))
  (Rendering|Material|SetScalarParameterValue (Variables|Default|GetDynMat) "illuminationIntensity" 0.0 :!class /Script/Engine.MaterialInstanceDynamic :!label _label)
  (Rendering|Components|Light|SetIntensity (Variables|Default|GetSpotLight10_0) 0.0)
  (Utilities|FlowControl|Delay _flickerduration)
  (Rendering|Material|SetScalarParameterValue (Variables|Default|GetDynMat) "illuminationIntensity" 4.0 :!class /Script/Engine.MaterialInstanceDynamic)
  (Rendering|Components|Light|SetIntensity (Variables|Default|GetSpotLight10_0) 2.5e+03)
  (Utilities|FlowControl|Delay _flickerduration)
  (Variables|Default|SetflickerCounter (+ (Variables|Default|GetflickerCounter) 1))
  (Math|Integer|CompareInt (Variables|Default|GetflickerCounter) 10
    (:>
      _)
    (:==
      _)
    (:<
      (goto _label)))
  (Rendering|Material|SetScalarParameterValue (Variables|Default|GetDynMat) "illuminationIntensity" 0.0 :!class /Script/Engine.MaterialInstanceDynamic)
  (Rendering|Components|Light|SetIntensity (Variables|Default|GetSpotLight10_0) 0.0))

(event EventBeginPlay)

(fn ConstructionScript
  (bind _returnvalue (Rendering|Material|CreateDynamicMaterialInstance (Variables|Default|GetDH_LVL_ArchLight_SM_0) 0 "/Game/Developers/SHASHANK/SciFi/Materials/ArchLight_Mat.ArchLight_Mat" :!class /Script/Engine.PrimitiveComponent))
  (Variables|Default|SetDynMat _returnvalue)
  (bind _returnvalue_2 (Rendering|Material|CreateDynamicMaterialInstance (Variables|Default|GetDH_LVL_ArchLight_SM_2_0) 0 "/Game/Developers/SHASHANK/SciFi/Materials/ArchLight_Mat.ArchLight_Mat" :!class /Script/Engine.PrimitiveComponent))
  (Variables|Default|SetDynMat_1 _returnvalue_2)
  (bind _returnvalue_3 (Rendering|Material|CreateDynamicMaterialInstance (Variables|Default|GetDH_LVL_ArchLight_SM_3_0) 0 "/Game/Developers/SHASHANK/SciFi/Materials/ArchLight_Mat.ArchLight_Mat" :!class /Script/Engine.PrimitiveComponent))
  (Variables|Default|SetDynMat_2 _returnvalue_3)
  (bind _returnvalue_4 (Rendering|Material|CreateDynamicMaterialInstance (Variables|Default|GetDH_LVL_ArchLight_SM_4_0) 0 "/Game/Developers/SHASHANK/SciFi/Materials/ArchLight_Mat.ArchLight_Mat" :!class /Script/Engine.PrimitiveComponent))
  (Variables|Default|SetDynMat_3 _returnvalue_4)
  (bind _returnvalue_5 (Rendering|Material|CreateDynamicMaterialInstance (Variables|Default|GetDH_LVL_ArchLight_SM_5_0) 0 "/Game/Developers/SHASHANK/SciFi/Materials/ArchLight_Mat.ArchLight_Mat" :!class /Script/Engine.PrimitiveComponent))
  (Variables|Default|SetDynMat_4 _returnvalue_5)
  (bind _returnvalue_6 (Rendering|Material|CreateDynamicMaterialInstance (Variables|Default|GetDH_LVL_ArchLight_SM_6_0) 0 "/Game/Developers/SHASHANK/SciFi/Materials/ArchLight_Mat.ArchLight_Mat" :!class /Script/Engine.PrimitiveComponent))
  (Variables|Default|SetDynMat_5 _returnvalue_6)
  (bind _returnvalue_7 (Rendering|Material|CreateDynamicMaterialInstance (Variables|Default|GetDH_LVL_ArchLight_SM_7_0) 0 "/Game/Developers/SHASHANK/SciFi/Materials/ArchLight_Mat.ArchLight_Mat" :!class /Script/Engine.PrimitiveComponent))
  (Variables|Default|SetDynMat_6 _returnvalue_7)
  (bind _returnvalue_8 (Rendering|Material|CreateDynamicMaterialInstance (Variables|Default|GetDH_LVL_ArchLight_SM_8_0) 0 "/Game/Developers/SHASHANK/SciFi/Materials/ArchLight_Mat.ArchLight_Mat" :!class /Script/Engine.PrimitiveComponent))
  (Variables|Default|SetDynMat_7 _returnvalue_8)
  (bind _returnvalue_9 (Rendering|Material|CreateDynamicMaterialInstance (Variables|Default|GetDH_LVL_ArchLight_SM_10_0) 0 "/Game/Developers/SHASHANK/SciFi/Materials/ArchLight_Mat.ArchLight_Mat" :!class /Script/Engine.PrimitiveComponent))
  (Variables|Default|SetDynMat_8 _returnvalue_9)
  (bind _returnvalue_10 (Rendering|Material|CreateDynamicMaterialInstance (Variables|Default|GetDH_LVL_ArchLight_SM_11_0) 0 "/Game/Developers/SHASHANK/SciFi/Materials/ArchLight_Mat.ArchLight_Mat" :!class /Script/Engine.PrimitiveComponent))
  (Variables|Default|SetDynMat_9 _returnvalue_10))